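; BP_FadeActor is an actor whose mesh fades out and back in through a material "Fade" parameter.
; The construction script caches the original materials and builds dynamic instances from a list of fade materials.
; FadeOut swaps in those instances by slot index and plays a timeline driving Fade, while Fadein reverses it.
; When the timeline finishes at 1 or above, the original materials are restored.
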(event `/Game/Blueprints/Actor/FadeActor/BI_FadeInterface.FadeOut`
  (`self.Set Materails to Dyanmic Instance`)
  (bind (_direction `_새_트랙_0`) (`Timeline|FadeTimeLine` :!via `PlayFromStart` :!label _label)
    (:`Update`
      (for _array_element (`self.DynamicMaterialIns`)
        (`MaterialInstanceDynamic.SetScalarParameterValue` _array_element "Fade" `_새_트랙_0`)))
    (:`Finished`
      (if (>= `_새_트랙_0` 1.0)
        (`self.ResetMaterail`)))))

(event `/Game/Blueprints/Actor/FadeActor/BI_FadeInterface.FadeIn`
  (goto _label :!via `Reverse`))

(event `self.ReceiveBeginPlay`)

(fn `ResetMaterail`
  (for (_array_element _array_index) (`self.OriginalMaterials`)
    (`PrimitiveComponent.SetMaterial` (`self.mESH`) _array_index _array_element)))

(fn `Set Materails to Dyanmic Instance`
  (for (_array_element _array_index) (`self.DynamicMaterialIns`)
    (`PrimitiveComponent.SetMaterial` (`self.mESH`) _array_index _array_element)))

(fn `UserConstructionScript`
  (`KismetArrayLibrary.Array_Clear` (`self.DynamicMaterialIns`))
  (set `self.OriginalMaterials` (`MeshComponent.GetMaterials` (`self.mESH`)))
  (for _array_element (`self.FadeMaterialInstance`)
    (bind _returnvalue (`KismetMaterialLibrary.CreateDynamicMaterialInstance` _array_element))
    (`KismetArrayLibrary.Array_AddUnique` (`self.DynamicMaterialIns`) _returnvalue)))