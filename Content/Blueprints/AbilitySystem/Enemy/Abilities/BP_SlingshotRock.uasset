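; Slingshot rock actor for an enemy ability, presumably thrown as a projectile, that tumbles as it moves.
; BeginPlay picks random yaw, pitch and roll rates, which Tick applies as frame-rate-independent local rotation on the static mesh.
; After a short delay, BeginPlay switches the sphere's collision to query-only.
; Movement and hit handling are not in this graph, and the overlap event is empty.
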(event `self.ReceiveBeginPlay`
  (bind _returnvalue (`KismetMathLibrary.RandomFloatInRange` -500.0 500.0))
  (set `self.Yaw Rotation Rate` _returnvalue)
  (set `self.PitchRoationRate` _returnvalue)
  (set `self.RollRotationRate` _returnvalue)
  (`KismetSystemLibrary.Delay` 0.1)
  (bind _sphere (`self.Sphere`)
    (:`then`
      (`PrimitiveComponent.SetCollisionEnabled` _sphere "QueryOnly"))
    (:`else`)))

(event `self.ReceiveTick`
  (params (DeltaSeconds :type "Float (single-precision)"))
  (`SceneComponent.K2_AddLocalRotation` (`self.StaticMesh`) (`KismetMathLibrary.MakeRotator` (* DeltaSeconds (`self.RollRotationRate`)) (* DeltaSeconds (`self.PitchRoationRate`)) (* DeltaSeconds (`self.Yaw Rotation Rate`))) false false))

(fn `UserConstructionScript`)